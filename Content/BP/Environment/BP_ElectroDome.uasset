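; BP_ElectroDome is an environment dome that repels dragons colliding with it, apparently acting as an electric boundary.
; On hit, it spawns a collision particle at the impact point, stops the dragon's movement and sets its player controller's InputMode to false.
; It then shoves the dragon far along the negated impact normal with an unswept world offset.
; A DoOnce, reset after a short delay, throttles repeated hits.
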(event `self.Dome.OnComponentHit`
  (params (HitComponent :type "PrimitiveComponent Object Reference") (OtherActor :type "Actor Object Reference") (OtherComp :type "PrimitiveComponent Object Reference") (NormalImpulse :type "Vector Structure") (Hit :type "HitResult Structure (by ref)"))
  (bind _asdragon_base (cast `/Game/BP/Dragons/DragonBase` OtherActor)
    (:`then`
      (`/Engine/EditorBlueprintResources/StandardMacros.DoOnce` false :!label _label
        (:`Completed`
          (bind _returnvalue (`GameplayStatics.SpawnEmitterAtLocation` "/Game/ArtAssets/EnvironmentalAssets/CollisionEffects/Dome_Collision.Dome_Collision" Hit_Location (`KismetMathLibrary.FindLookAtRotation` Hit_Location (+ Hit_Normal Hit_ImpactNormal))))
          (`ActorComponent.SetActive` _returnvalue true false)
          (`MovementComponent.StopMovementImmediately` (`Character.CharacterMovement` _asdragon_base))
          (bind _asdragon_player_controller (cast `/Game/BP/Dragons/DragonPlayerController` (`Pawn.GetController` _asdragon_base))
            (:`then`
              (set `/Game/BP/Dragons/DragonPlayerController.InputMode` false _asdragon_player_controller))
            (:`CastFailed`
              _)))))
    (:`CastFailed`
      _))
  (`self.K2_AddActorWorldOffset` _asdragon_base (* Hit_ImpactNormal -5000) false false)
  (`KismetSystemLibrary.Delay` 0.3)
  (goto _label :!via `Reset`))

(fn `UserConstructionScript`)